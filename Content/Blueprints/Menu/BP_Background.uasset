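; BP_Background is a menu background actor that displays an HDRI cubemap on a sphere and slowly rotates it.
; The construction script turns off the sphere's shadow casting, collision and character step-up.
; BeginPlay creates a dynamic instance of MI_HDRI_Master on the sphere, and Tick advances its CubemapRotation parameter by RotationSpeed scaled by delta time, so the material animates without moving the mesh.
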(event `self.ReceiveBeginPlay`
  (bind _returnvalue (`PrimitiveComponent.CreateDynamicMaterialInstance` (`self.Sphere`) 0 "/Game/Assets/HDRI/MI_HDRI_Master.MI_HDRI_Master" "None"))
  (set `self.MaterialDynamicInstanceRef` _returnvalue))

(event `self.ReceiveTick`
  (params (DeltaSeconds :type "Float (single-precision)"))
  (bind _materialdynamicinstanceref (`self.MaterialDynamicInstanceRef`))
  (bind _returnvalue (`MaterialInstanceDynamic.K2_GetScalarParameterValue` _materialdynamicinstanceref "CubemapRotation"))
  (`MaterialInstanceDynamic.SetScalarParameterValue` _materialdynamicinstanceref "CubemapRotation" (+ _returnvalue (* DeltaSeconds (`self.RotationSpeed`)))))

(fn `UserConstructionScript`
  (bind _sphere (`self.Sphere`))
  (`PrimitiveComponent.SetCastShadow` (`self.Sphere`) false)
  (`PrimitiveComponent.SetCollisionProfileName` _sphere "NoCollision" true)
  (set `PrimitiveComponent.CanCharacterStepUpOn` "ECB_No" _sphere))