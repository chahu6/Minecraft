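; Test Geometry Script actor that procedurally builds a box wall with a hole cut into it.
; The Construction Script resets the dynamic mesh, appends the wall box, creates a random stream from Seed, then calls AddHole once.
; AddHole places a default-sized box at a seeded random point on a pooled compute mesh, boolean-subtracts it from the wall, then releases the compute meshes.
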(fn `AddHole`
  (bind _returnvalue (`self.AllocateComputeMesh`))
  (bind _returnvalue_2 (`GeometryScriptLibrary_MeshPrimitiveFunctions.AppendBox` _returnvalue (struct) (`KismetMathLibrary.MakeTransform` (`KismetMathLibrary.RandomPointInBoundingBoxFromStream` (`self.Random`) (0.0 0.0 0.0) (25.0 75.0 100.0))) 100.0 100.0 100.0 0 0 0 "Base" null))
  (bind _returnvalue_3 (`BaseDynamicMeshComponent.GetDynamicMesh` (`self.DynamicMeshComponent`)))
  (`GeometryScriptLibrary_MeshBooleanFunctions.ApplyMeshBoolean` _returnvalue_3 (struct) _returnvalue_2 (struct) "Subtract" (struct) null)
  (`self.ReleaseAllComputeMeshes`))

(fn `UserConstructionScript`
  (bind _returnvalue (`BaseDynamicMeshComponent.GetDynamicMesh` (`self.DynamicMeshComponent`)))
  (bind _returnvalue_2 (`DynamicMesh.Reset` _returnvalue))
  (`GeometryScriptLibrary_MeshPrimitiveFunctions.AppendBox` _returnvalue_2 (struct) (struct) 100.0 500.0 300.0 0 0 0 "Base" null)
  (set `self.Random` (`KismetMathLibrary.MakeRandomStream` (`self.Seed`)))
  (`self.AddHole`))